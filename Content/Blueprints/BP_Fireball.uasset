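; Fireball hazard that waits hidden until a pawn enters its capsule, then drops toward a static mesh on the ground.
; BeginPlay randomly offsets the fireball upward; the trigger moves it down over a random fall time and destroys the actor on arrival.
; Partway through the fall, scaled by AlertFactor, the mesh swaps material.
; A pawn touching the fireball deals one damage to player 0's BP_MyPS and destroys the actor.
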(event `self.ReceiveBeginPlay`
  (`SceneComponent.K2_AddRelativeLocation` (`self.fireball`) (`KismetMathLibrary.MakeVector` (`KismetMathLibrary.RandomFloatInRange` -200.0 -300.0) (`KismetMathLibrary.RandomFloatInRange` 300.0 400.0) (`KismetMathLibrary.RandomFloatInRange` 700.0 800.0)) false false)
  (`self.SetActorHiddenInGame` true))

(event `self.Capsule.OnComponentBeginOverlap`
  (params (OverlappedComponent :type "PrimitiveComponent Object Reference") (OtherActor :type "Actor Object Reference") (OtherComp :type "PrimitiveComponent Object Reference") (OtherBodyIndex :type Integer) (bFromSweep :type Boolean) (SweepResult :type "HitResult Structure (by ref)"))
  (bind _falltimerange (`self.FallTimeRange`))
  (cast `Pawn` OtherActor)
  (`self.SetActorHiddenInGame` false)
  (set `self.FallTime` (`KismetMathLibrary.RandomFloatInRange` (`.Value` (break `FloatRangeBound` (break `FloatRange` _falltimerange))) (`.Value` (break `FloatRangeBound` (`.UpperBound` (break `FloatRange` _falltimerange))))))
  (`|ExecutionSequence`
    (:`then_0`
      (`KismetSystemLibrary.MoveComponentTo` (`self.fireball`) (`SceneComponent.RelativeLocation` (`self.StaticMesh`)) (struct) false false (`self.FallTime`))
      (`self.K2_DestroyActor`))
    (:`then_1`
      (`KismetSystemLibrary.Delay` (* (`self.FallTime`) (`self.AlertFactor`)))
      (`PrimitiveComponent.SetMaterial` (`self.StaticMesh`) 0 "/Engine/MapTemplates/Materials/BasicAsset01.BasicAsset01"))))

(event `self.fireball.OnComponentBeginOverlap`
  (params (OverlappedComponent :type "PrimitiveComponent Object Reference") (OtherActor :type "Actor Object Reference") (OtherComp :type "PrimitiveComponent Object Reference") (OtherBodyIndex :type Integer) (bFromSweep :type Boolean) (SweepResult :type "HitResult Structure (by ref)"))
  (cast `Pawn` OtherActor)
  (bind _asbp_my_ps (cast `/Game/Blueprints/BP_MyPS` (`GameplayStatics.GetPlayerState` 0)))
  (`/Game/Blueprints/BP_MyPS.TakeDamage` _asbp_my_ps 1)
  (`self.K2_DestroyActor`))

(fn `UserConstructionScript`)