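; BP_Bird is a player-controlled bird pawn for a 2D mode, with movement, energy-limited flight and interaction through Enhanced Input.
; BeginPlay swaps in the 2D mapping contexts, finds or spawns BP_Camera_2D as view target and fills energy.
; Holding fly disables mesh gravity and climbs while draining energy, then descends at glide speed when empty; energy recovers otherwise.
; Tick applies accumulated movement input through unswept SetActorLocation, without delta-time scaling.
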(event `self.ReceiveTick`
  (params (DeltaSeconds :type "Float (single-precision)"))
  (`|ExecutionSequence`
    (:`then_0`
      (if (`self.Flying`)
        (if (> (`self.CurEnergy`) 0.0)
          (`self.AddMovementInput` (`KismetMathLibrary.GetUpVector` (struct)) (`self.FlySpeed`))
          (bind _output_get (set `self.CurEnergy` (`KismetMathLibrary.FMax` (- (`self.CurEnergy`) DeltaSeconds))))
          (`KismetSystemLibrary.PrintString` (`KismetStringLibrary.Conv_DoubleToString` _output_get))
          (else
            (`self.AddMovementInput` (`KismetMathLibrary.GetUpVector` (struct)) (* (`self.GlideSpeed`) -1.0))))
        (else
          (`self.RecoverEnergy` DeltaSeconds))))
    (:`then_1`
      (`self.UpdatePos`))))

(event `self.ReceiveBeginPlay`
  ;[1 1 1] Input
  (bind _asplayer_controller (cast `PlayerController` (`self.GetController`)))
  (bind _returnvalue (pcsubsystem `EnhancedInputLocalPlayerSubsystem` _asplayer_controller))
  (`/Engine/EditorBlueprintResources/StandardMacros.IsValid` _returnvalue
    (:`Is Valid`
      (`EnhancedInputSubsystemInterface.ClearAllMappings` _returnvalue)
      (`EnhancedInputSubsystemInterface.AddMappingContext` _returnvalue "/Game/Input/IMC_2D.IMC_2D" 0 (struct))
      (`EnhancedInputSubsystemInterface.AddMappingContext` _returnvalue "/Game/Input/IMC_2D_Bird.IMC_2D_Bird" 0 (struct))
      ;[1 1 1] Camera
      (bind _outactors (`GameplayStatics.GetAllActorsOfClass` "/Game/Blueprints/BP_Camera_2D.BP_Camera_2D_C"))
      (if (not (`KismetArrayLibrary.Array_IsEmpty` _outactors))
        (set `self.2DCamera` (`|GetArrayItem` _outactors))
        (else
          (bind _returnvalue_2 (`|SpawnActorFromClass` "/Game/Blueprints/BP_Camera_2D.BP_Camera_2D_C" (`KismetMathLibrary.MakeTransform` (`self.K2_GetActorLocation`)) "Undefined" "MultiplyWithRoot" null self null))
          (set `self.2DCamera` _returnvalue_2)))
      (`PlayerController.SetViewTargetWithBlend` (`GameplayStatics.GetPlayerController` 0) (`self.2DCamera`) 0.0 "VTBlend_Linear" 1.0 false)
      (set `self.CurEnergy` (`self.MaxEnergy`)))))

(event `EnhancedInput|/Game/Input/Actions/IA_Move_2D`
  (params (ActionValue :type "Float (double-precision)") (ElapsedSeconds :type "Float (double-precision)") (TriggeredSeconds :type "Float (double-precision)") (InputAction :type "InputAction Object Reference" :default "/Game/Input/Actions/IA_Move_2D.IA_Move_2D"))
  (bind (_returnvalue_roll _returnvalue_pitch _returnvalue_yaw) (`KismetMathLibrary.BreakRotator` (`self.GetControlRotation`)))
  (:`Triggered`
    (`self.AddMovementInput` (`KismetMathLibrary.GetForwardVector` (`KismetMathLibrary.MakeRotator` 0.0 0.0 _returnvalue_yaw)) (* (`self.MoveSpeed`) ActionValue))))

(event `EnhancedInput|/Game/Input/Actions/IA_Interact`
  (params (ActionValue :type Boolean) (ElapsedSeconds :type "Float (double-precision)") (TriggeredSeconds :type "Float (double-precision)") (InputAction :type "InputAction Object Reference" :default "/Game/Input/Actions/IA_Interact.IA_Interact"))
  (bind _interact_target (`self.Interact Target`))
  (:`Triggered`
    (if (`KismetSystemLibrary.IsValidInterface` _interact_target)
      (`/Game/Blueprints/IInteractable.Interact` _interact_target))))

(event `EnhancedInput|/Game/Input/Actions/IA_Fly`
  (params (ActionValue :type Boolean) (ElapsedSeconds :type "Float (double-precision)") (TriggeredSeconds :type "Float (double-precision)") (InputAction :type "InputAction Object Reference" :default "/Game/Input/Actions/IA_Fly.IA_Fly"))
  (:`Triggered`
    (bind _output_get (set `self.Flying` ActionValue))
    (`PrimitiveComponent.SetEnableGravity` (`self.StaticMesh`) (not _output_get))))

(fn `RecoverEnergy`
  (params (Recover :type "Float (double-precision)"))
  (if (< (`self.CurEnergy`) (`self.MaxEnergy`))
    (set `self.CurEnergy` (`KismetMathLibrary.FMin` (+ (`self.CurEnergy`) (* Recover (`self.EnergyRecoverRate`))) (`self.MaxEnergy`)))))

(fn `UpdatePos`
  (bind _returnvalue (`self.ConsumeMovementInputVector`))
  (`self.K2_SetActorLocation` (+ _returnvalue (`self.K2_GetActorLocation`))))

(fn `UserConstructionScript`)