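; BP_Camera_2D is a camera actor, named for 2D use, that smoothly follows a target actor.
; Every tick, UpdateCameraPos interpolates the actor's location toward FollowTarget with VInterpTo at InterpSpeed and moves it without sweep.
; When LockHeight is set, the target Z is world zero instead of the followed actor's height.
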(event `self.ReceiveTick`
  (params (DeltaSeconds :type "Float (single-precision)"))
  (`self.UpdateCameraPos`))

(fn `UpdateCameraPos`
  (locals (LockHeight :type Boolean))
  (bind (_returnvalue_x _returnvalue_y _returnvalue_z) (`KismetMathLibrary.BreakVector` (`self.K2_GetActorLocation`)))
  (bind (_returnvalue_x_2 _returnvalue_y_2 _returnvalue_z_2) (`KismetMathLibrary.BreakVector` (`self.K2_GetActorLocation` (`self.FollowTarget`))))
  (`self.K2_SetActorLocation` (`KismetMathLibrary.VInterpTo` (`KismetMathLibrary.MakeVector` _returnvalue_x _returnvalue_y _returnvalue_z) (`KismetMathLibrary.MakeVector` _returnvalue_x_2 _returnvalue_y_2 (select `bool` (`local.LockHeight`) :`false` _returnvalue_z_2)) (`GameplayStatics.GetWorldDeltaSeconds`) (`self.Interp Speed`))))

(fn `UserConstructionScript`)