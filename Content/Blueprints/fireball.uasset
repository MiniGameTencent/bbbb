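; Falling fireball hazard actor that appears after a random delay, drops toward its static mesh and damages players.
; On BeginPlay it offsets the Fireball component randomly upward and sideways, stays hidden, then eases it down over a random fall time.
; Near the end of the fall it swaps the mesh material and sets IsOnfire, then destroys itself shortly after.
; Capsule overlap damages pawns through their BP_MyPS player state, without checking IsOnfire.
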(event `self.ReceiveBeginPlay`
  (set `self.wait_time` (`KismetMathLibrary.RandomFloatInRange` 0.0 10.0))
  (set `self.is_onfire` false)
  (`SceneComponent.K2_AddRelativeLocation` (`self.fireball`) (`KismetMathLibrary.MakeVector` (`KismetMathLibrary.RandomFloatInRange` 100.0 1000.0) (`KismetMathLibrary.RandomFloatInRange` 100.0 1000.0) (`KismetMathLibrary.RandomFloatInRange` 1500.0 2000.0)) false false)
  (`self.SetActorHiddenInGame` true)
  (`KismetSystemLibrary.Delay` (`self.wait_time`))
  (`self.SetActorHiddenInGame` false)
  (bind _output_get (set `self.fall_time` (`KismetMathLibrary.RandomFloatInRange` 1.0 3.0)))
  (`|ExecutionSequence`
    (:`then_0`
      (`KismetSystemLibrary.MoveComponentTo` (`self.fireball`) (- (`KismetMathLibrary.MakeVector` (.x (`SceneComponent.RelativeLocation` (`self.StaticMesh`))) (.y (`SceneComponent.RelativeLocation` (`self.StaticMesh`))) (+ (.z (`SceneComponent.RelativeLocation` (`self.StaticMesh`))) 200.0)) (`SceneComponent.RelativeLocation` (`self.fireball`))) (struct) false true _output_get))
    (:`then_1`
      (`KismetSystemLibrary.Delay` (* _output_get 0.8))
      (`PrimitiveComponent.SetMaterial` (`self.StaticMesh`) 0 "/Engine/MapTemplates/Materials/BasicAsset01.BasicAsset01")
      (set `self.is_onfire` true)
      (`KismetSystemLibrary.Delay` (`KismetMathLibrary.RandomFloatInRange` 2.0 5.0))
      (`self.K2_DestroyActor`))))

(event `self.Capsule.OnComponentBeginOverlap`
  (params (OverlappedComponent :type "PrimitiveComponent Object Reference") (OtherActor :type "Actor Object Reference") (OtherComp :type "PrimitiveComponent Object Reference") (OtherBodyIndex :type Integer) (bFromSweep :type Boolean) (SweepResult :type "HitResult Structure (by ref)"))
  (bind _aspawn (cast `Pawn` OtherActor))
  (bind _asbp_my_ps (cast `/Game/Blueprints/BP_MyPS` (`Pawn.PlayerState` _aspawn)))
  (`/Game/Blueprints/BP_MyPS.TakeDamage` _asbp_my_ps (`self.damage`)))

(fn `UserConstructionScript`)